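; Map generation component that builds a stage's node map column by column from the rules in a StageDataAsset.
; Start rules create a single room widget from RoomTypeTable, add it to NodeSet and mark it as the player location, with gates to catch conflicting rules.
; Middle rules loop toward a reserved last column, but only second-column height sizing is sketched.
; End rules and node creation beyond the start are absent, and the seeded density roll is unwired.
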(fn `GenerateNodes`
  (params (StageDataAsset :type "/Game/MapSystem/DataAssets/StageDataAsset Object Reference"))
  (locals (NodeSet :type "Set of /Game/MapSystem/Structs/NodeGenerationStruct Structure") (RoomTypeTable :type "DataTable Object Reference" :default "/Script/Engine.DataTable'/Game/MapSystem/Widgets/MapNode/RoomTypeTable.RoomTypeTable'") (ColumnIndex :type Integer :default 0) (TmpColumnHeight :type Integer) (GameModeRef :type "/Game/GameModes/MainGameMode Object Reference"))
  (`|ExecutionSequence`
    (:`then_0`
      (bind _asmain_game_mode (cast `/Game/GameModes/MainGameMode` (`GameplayStatics.GetGameMode`)))
      (set `local.GameModeRef` _asmain_game_mode))
    (:`then_1`
      (set `self.MapHeight` 0)
      (set `local.TmpColumnHeight` 0)
      (set `local.ColumnIndex` 0)
      (`|ExecutionSequence`
        (:`then_0`
          (if (`BlueprintSetLibrary.Set_Contains` (`/Game/MapSystem/DataAssets/StageDataAsset.MapRules` (`local.StageDataAsset`)) "NewEnumerator0")
            (`|ExecutionSequence`
              (:`then_0`
                (`/Engine/EditorBlueprintResources/StandardMacros.Gate` true :!label _label
                  (:`Exit`
                    (`KismetSystemLibrary.PrintString` "error:More than one Start generation rule active"))))
              (:`then_1`
                (goto _label :!via `Open`))
              (:`then_2`
                (bind _returnvalue (`|GetDataTableRow` (`local.RoomTypeTable`) "StartRoom")
                  (:`then`
                    (bind _returnvalue_2 (`|CreateWidget` "/Game/MapSystem/Widgets/MapNode/MapNodeWidget.MapNodeWidget_C" null _returnvalue))
                    (`BlueprintSetLibrary.Set_Add` (`local.NodeSet`) (make `/Game/MapSystem/Structs/NodeGenerationStruct` _returnvalue_2 (`local.ColumnIndex`)))
                    (`self.ValidateMapHeight` 1))
                  (:`RowNotFound`
                    (`KismetSystemLibrary.PrintString` "error:Requested row from RoomTypeTable was not found")))))))
        (:`then_1`
          (`|ExecutionSequence`
            (:`then_0`
              (`/Engine/EditorBlueprintResources/StandardMacros.IncrementInt` (`local.ColumnIndex`)))
            (:`then_1`
              (bind _result (`BlueprintSetLibrary.Set_ToArray` (`local.NodeSet`)))
              (`/Game/MapSystem/Widgets/MapNode/MapNodeWidget.TogglePlayerLocation` (`.NodeWidget_2_116609834EBAE0936CE12185421E2C13` (break `/Game/MapSystem/Structs/NodeGenerationStruct` (`|GetArrayItem` _result))) true))))))
    (:`then_2`
      (while (< (`local.ColumnIndex`) (- (`/Game/MapSystem/DataAssets/StageDataAsset.StageLength` (`local.StageDataAsset`)) 1 1))
        (`|ExecutionSequence`
          (:`then_0`
            (if (== (`local.ColumnIndex`) 1)
              (`|ExecutionSequence`
                (:`then_0`
                  (`/Engine/EditorBlueprintResources/StandardMacros.Gate` false
                    (:`Exit`
                      (if (`BlueprintSetLibrary.Set_Contains` (`/Game/MapSystem/DataAssets/StageDataAsset.MapRules` (`local.StageDataAsset`)) "NewEnumerator2")
                        (`|ExecutionSequence`
                          (:`then_0`
                            (bind _output_get (set `local.TmpColumnHeight` (`self.RandomColumnDensity`)))
                            (`self.ValidateMapHeight` _output_get)))))))))))))))